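; Spline prop scatterer for the sports stadium that fills rows of a chosen static mesh, such as tiered seating, at construction time.
; The construction script steps along the spline at fixed spacing, adding hierarchical instances in local space with spline yaw plus an extra rotation.
; Each row is offset by depth on local Y, not perpendicular to the spline, and raised by height.
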(fn `UserConstructionScript`
  (bind _returnvalue (* (`self.CurrentIndex`) (`self.Spacing`)))
  (bind (_returnvalue_x _returnvalue_y _returnvalue_z) (`KismetMathLibrary.BreakVector` (`SplineComponent.GetLocationAtDistanceAlongSpline` (`self.Spline`) _returnvalue "Local")))
  (bind (_returnvalue_roll _returnvalue_pitch _returnvalue_yaw) (`KismetMathLibrary.BreakRotator` (`SplineComponent.GetRotationAtDistanceAlongSpline` (`self.Spline`) _returnvalue "Local")))
  (`StaticMeshComponent.SetStaticMesh` (`self.HierarchicalInstancedStaticMesh`) (`self.Mesh`)) ; Set the static mesh for the base of the legs
  (for _index (range (+ (`self.Column`) 1))
    (set `self.CurrentIndex` _index)
    (for _index_2 (range (`self.Raw`))
      (`InstancedStaticMeshComponent.AddInstance` (`self.HierarchicalInstancedStaticMesh`) (`KismetMathLibrary.MakeTransform` (`KismetMathLibrary.MakeVector` _returnvalue_x (+ (* _index_2 (`self.Depth`)) _returnvalue_y) (+ (* _index_2 (`self.Height`)) _returnvalue_z)) (`KismetMathLibrary.MakeRotator` 0.0 0.0 (+ _returnvalue_yaw (`self.AddRotation`)))) false))))