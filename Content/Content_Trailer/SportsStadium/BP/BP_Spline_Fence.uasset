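; Spline-based fence tool that lays copies of a mesh along an editable spline, apparently for the sports stadium level.
; The construction script derives the section count from spline length divided by mesh width plus a spacing adjustment.
; Sections become hierarchical instanced mesh instances, yawed to the spline at an adjustable distance offset, without pitch or roll.
; The final position gets a separate static mesh component when an optional end mesh is set.
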(fn `UserConstructionScript`
  (bind _mesh (`self.Mesh`))
  (bind _spline (`self.Spline`))
  (bind _endmesh (`self.EndMesh`))
  (bind _returnvalue (+ (* (.x (`.BoxExtent` (`KismetMathLibrary.BreakBoxSphereBounds` (`StaticMesh.GetBounds` _mesh)))) 2.0) (`self.SpacingAdjustment`)))
  (bind _returnvalue_2 (* (`self.CurrentIndex`) _returnvalue))
  (bind (_returnvalue_x _returnvalue_y _returnvalue_z) (`KismetMathLibrary.BreakVector` (`SplineComponent.GetLocationAtDistanceAlongSpline` _spline _returnvalue_2 "Local")))
  (bind (_returnvalue_roll _returnvalue_pitch _returnvalue_yaw) (`KismetMathLibrary.BreakRotator` (`SplineComponent.GetRotationAtDistanceAlongSpline` _spline (+ _returnvalue_2 (`self.RotationAdjust`)) "Local")))
  (bind _returnvalue_3 (`KismetMathLibrary.MakeTransform` (`KismetMathLibrary.MakeVector` _returnvalue_x _returnvalue_y _returnvalue_z) (`KismetMathLibrary.MakeRotator` 0.0 0.0 _returnvalue_yaw)))
  (`StaticMeshComponent.SetStaticMesh` (`self.HierarchicalInstancedStaticMesh`) _mesh) ; Set the static mesh for the base of the legs
  (bind _output_get (set `self.InstanceNum` (`KismetMathLibrary.FTrunc` (/ (`SplineComponent.GetSplineLength` (`self.Spline`)) _returnvalue))))
  (for _index (range (+ _output_get 1))
    (set `self.CurrentIndex` _index)
    (if (!= (`self.InstanceNum`) (`self.CurrentIndex`))
      (`InstancedStaticMeshComponent.AddInstance` (`self.HierarchicalInstancedStaticMesh`) _returnvalue_3 false)
      (else
        (`/Engine/EditorBlueprintResources/StandardMacros.IsValid` _endmesh
          (:`Is Valid`
            (bind _returnvalue_4 (`AddComponent|NODE_AddStaticMeshComponent-1` :`RelativeTransform` _returnvalue_3))
            (`StaticMeshComponent.SetStaticMesh` _returnvalue_4 _endmesh)))))))